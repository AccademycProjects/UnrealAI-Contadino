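; Turret pawn that aims at a given target and shows its state on an andon light.
; Aiming smoothly interpolates actor yaw toward the target and pitches a separate pivot within clamped limits, both at RotationSpeed.
; A child-actor andon light, cached on BeginPlay, changes color for Disabled, Active and Alert states.
; Simple getters expose the active and enabled flags.
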(event `self.ReceiveBeginPlay`
  (bind _asbp_andon_light (cast `/Game/Farmer/Blueprint/BP_AndonLight` (`ChildActorComponent.ChildActor` (`self.BP_AndonLight`))))
  (set `self.AndonLightRef` _asbp_andon_light))

(event `ChangeState`
  (params (NewState :type "/Game/Farmer/Blueprint/ETurretState Enum" :default "NewEnumerator0"))
  (`/Game/Farmer/Blueprint/BP_AndonLight.ChangeColor` (`self.AndonLightRef`) (select `/Game/Farmer/Blueprint/ETurretState` NewState :`NewEnumerator0` (struct :`R` 0.14996 :`G` 0.14996 :`B` 0.14996 :`A` 1.0) :`NewEnumerator1` (struct :`R` 1.0 :`A` 1.0) :`NewEnumerator2` (struct :`G` 1.0 :`B` 1.0 :`A` 1.0) :!type "LinearColor Structure")))

(fn `Aiming`
  (params (Target :type "Actor Object Reference") (DeltaSeconds :type "Float (double-precision)"))
  (bind _returnvalue (`self.K2_GetActorLocation`))
  (bind _returnvalue_2 (`self.K2_GetActorLocation` Target))
  (bind _pivoty (`self.PivotY`))
  (bind (_returnvalue_roll _returnvalue_pitch _returnvalue_yaw) (`KismetMathLibrary.BreakRotator` (`KismetMathLibrary.FindLookAtRotation` _returnvalue _returnvalue_2)))
  (bind (_returnvalue_roll_2 _returnvalue_pitch_2) (`KismetMathLibrary.BreakRotator` (`KismetMathLibrary.Conv_VectorToRotator` (`KismetMathLibrary.Normal` (- _returnvalue_2 _returnvalue)))))
  (`self.K2_SetActorRotation` (`KismetMathLibrary.RInterpTo` (`self.K2_GetActorRotation`) (`KismetMathLibrary.MakeRotator` 0.0 0.0 _returnvalue_yaw) DeltaSeconds (`self.RotationSpeed`)))
  (`SceneComponent.K2_SetRelativeRotation` _pivoty (`KismetMathLibrary.RInterpTo` (`SceneComponent.RelativeRotation` _pivoty) (`KismetMathLibrary.MakeRotator` 0.0 (`KismetMathLibrary.ClampAngle` _returnvalue_pitch_2 -20.0 30.0)) DeltaSeconds (`self.RotationSpeed`)) false false))

(fn `IsActive`
  (returns (IsActive :type Boolean))
  (return (`self.Is Active`)))

(fn `IsEnable`
  (returns (IsEnable :type Boolean))
  (return (`self.Is Enable`)))

(fn `UserConstructionScript`)