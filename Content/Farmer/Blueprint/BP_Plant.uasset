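; BP_Plant is a farm plant actor that grows over time and becomes harvestable.
; On BeginPlay a timeline scales the root from a tenth to full size, recoloring the bush from brown to yellow once past halfway and to green when finished, when it sets Harvestable.
; Color changes go through a dynamic material instance created in the construction script and driven by the Color parameter.
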(event `self.ReceiveBeginPlay`
  (`self.ChangeColor` (struct :`R` 0.057972 :`G` 0.028181 :`B` 0.000839 :`A` 1.0))
  (`SceneComponent.SetRelativeScale3D` (`self.DefaultSceneRoot`) (0.1 0.1 0.1))
  (bind (_direction _growtime) (`Timeline|TL_Grow`)
    (:`Update`
      (`SceneComponent.SetRelativeScale3D` (`self.DefaultSceneRoot`) (`KismetMathLibrary.Conv_DoubleToVector` (`KismetMathLibrary.Lerp` 0.1 1.0 _growtime)))
      (if (and (not (`self.bHalfMaterialApplied`)) (> _growtime 0.5))
        (set `self.bHalfMaterialApplied` true)
        (`self.ChangeColor` (struct :`R` 1.0 :`G` 0.665972 :`A` 1.0))))
    (:`Finished`
      (set `self.bHarvestable` true)
      (`self.ChangeColor` (struct :`G` 1.0 :`A` 1.0)))))

(fn `ChangeColor`
  (params (Value :type "LinearColor Structure"))
  (bind _materialref (`self.MaterialRef`))
  (`MaterialInstanceDynamic.SetVectorParameterValue` _materialref "Color" Value)
  (`PrimitiveComponent.SetMaterial` (`self.CubyBush_Dark`) 0 _materialref))

(fn `UserConstructionScript`
  (bind _cubybush_dark (`self.CubyBush_Dark`))
  (bind _returnvalue (`PrimitiveComponent.CreateDynamicMaterialInstance` _cubybush_dark 0 (`PrimitiveComponent.GetMaterial` _cubybush_dark 0) "None"))
  (set `self.MaterialRef` _returnvalue))