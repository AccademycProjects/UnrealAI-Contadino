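; Farm plot actor that a BPPZ_Base instigator interacts with to sow and harvest plants.
; An empty plot spends one of the instigator's seeds to spawn a BP_Plant; a harvestable plant is destroyed and adds to their plant count.
; CanInteract always allows interaction, with no seed count check.
; GetStateTags exposes the plot as Sowable, Busy or Harvestable through AI state gameplay tags.
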(event `/Game/Farmer/Blueprint/BPI_Interactable.Interact`
  (params (Instigator :type "Pawn Object Reference"))
  (bind _currentplant (`self.CurrentPlant`))
  (bind _caninteract (`self.CanInteract` Instigator))
  (if _caninteract
    (bind _asbppz_base (cast `/Game/Farmer/Blueprint/BPPZ_Base` Instigator))
    (`/Engine/EditorBlueprintResources/StandardMacros.IsValid` _currentplant
      (:`Is Valid`
        (if (`/Game/Farmer/Blueprint/BP_Plant.bHarvestable` _currentplant)
          ; Harvest
          (`self.K2_DestroyActor` (`self.CurrentPlant`))
          (set `self.CurrentPlant` null)
          (`/Engine/EditorBlueprintResources/StandardMacros.IncrementInt` (`/Game/Farmer/Blueprint/BPPZ_Base.PlantsCount` _asbppz_base))))
      (:`Is Not Valid`
        ; Sowing
        (`/Engine/EditorBlueprintResources/StandardMacros.DecrementInt` (`/Game/Farmer/Blueprint/BPPZ_Base.SeedsCount` _asbppz_base)
          (:`  `
            (bind _returnvalue (`|SpawnActorFromClass` "/Game/Farmer/Blueprint/BP_Plant.BP_Plant_C" (`SceneComponent.K2_GetComponentToWorld` (`self.Spawn`)) "AlwaysSpawn" "MultiplyWithRoot" null null))
            (set `self.CurrentPlant` _returnvalue)))))))

(fn `CanInteract`
  (params (Instigator :type "Pawn Object Reference"))
  (returns (CanInteract :type Boolean))
  (return true))

(fn `GetStateTags`
  (returns (OutTags :type "GameplayTagContainer Structure"))
  (bind _currentplant (`self.CurrentPlant`))
  (`/Engine/EditorBlueprintResources/StandardMacros.IsValid` _currentplant
    (:`Is Valid`
      (return (select `bool` (`/Game/Farmer/Blueprint/BP_Plant.bHarvestable` _currentplant) :`false` (struct :`GameplayTags` (struct :`(TagName` "Consegna.AI.State.Farm.Busy"))) :`true` (struct :`GameplayTags` (struct :`(TagName` "Consegna.AI.State.Farm.Harvestable"))) :!type "GameplayTagContainer Structure")))
    (:`Is Not Valid`
      (return (struct :`GameplayTags` (struct :`(TagName` "Consegna.AI.State.Farm.Sowable")))))))

(fn `UserConstructionScript`)