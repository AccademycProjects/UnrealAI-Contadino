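; Base Blueprint for a farmer in a farming loop, showing a sprite and an andon status light.
; On BeginPlay it caches the player camera, starts a looping timer and gets the BP_AndonLight from a child actor component.
; ChangeState recolors that light for each task: taking seeds, sowing, harvesting or depositing plants.
; SetSpriteRotation billboards the sprite toward the camera on yaw only.
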(event `self.ReceiveBeginPlay`
  (bind _returnvalue (`GameplayStatics.GetPlayerController` 0))
  (`/Engine/EditorBlueprintResources/StandardMacros.IsValid` _returnvalue
    (:`Is Valid`
      (set `self.PlayerRef` _returnvalue)
      (set `self.CameraRef` (`PlayerController.PlayerCameraManager` _returnvalue))
      (`KismetSystemLibrary.K2_SetTimerDelegate` (`|CreateDelegate` :!event `SetSpriteRotation`) 0.2 true true)
      (bind _asbp_andon_light (cast `/Game/Farmer/Blueprint/BP_AndonLight` (`ChildActorComponent.ChildActor` (`self.BP_AndonLight`))))
      (set `self.AndonLightRef` _asbp_andon_light))))

(event `ChangeState`
  (params (State :type "/Game/Farmer/Blueprint/Enum/FarmerState Enum" :default "NewEnumerator0"))
  (`/Game/Farmer/Blueprint/BP_AndonLight.ChangeColor` (`self.AndonLightRef`) (select `/Game/Farmer/Blueprint/Enum/FarmerState` State :`NewEnumerator0` (struct :`R` 1.0 :`A` 1.0) :`NewEnumerator1` (struct :`R` 1.0 :`B` 1.0 :`A` 1.0) :`NewEnumerator2` (struct :`B` 1.0 :`A` 1.0) :`NewEnumerator3` (struct :`R` 1.0 :`G` 1.0 :`A` 1.0) :!type "LinearColor Structure")))

(fn `SetSpriteRotation`
  (`SceneComponent.K2_SetWorldRotation` (`self.Sprite`) (`KismetMathLibrary.MakeRotator` 0.0 0.0 (+ (.yaw (`KismetMathLibrary.FindLookAtRotation` (`SceneComponent.K2_GetComponentLocation` (`self.Sprite`)) (`PlayerCameraManager.GetCameraLocation` (`self.CameraRef`)))) 90.0)) false false))

(fn `UserConstructionScript`)