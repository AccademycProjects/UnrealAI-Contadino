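; BP_AndonLight is an andon indicator light whose Cube mesh changes color on request.
; The construction script creates a dynamic material instance from the Cube's first material and caches it in MaterialRef.
; The ChangeColor event skips repeat colors, otherwise stores the new color, sets the material's Color parameter and reapplies it to the Cube.
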(event `ChangeColor`
  (params (NewColor :type "LinearColor Structure"))
  (bind _materialref (`self.MaterialRef`))
  (if (!= (`self.CurrentColor`) NewColor)
    (set `self.CurrentColor` NewColor)
    (`MaterialInstanceDynamic.SetVectorParameterValue` _materialref "Color" NewColor)
    (`PrimitiveComponent.SetMaterial` (`self.Cube`) 0 _materialref)))

(fn `UserConstructionScript`
  (bind _cube (`self.Cube`))
  (bind _returnvalue (`PrimitiveComponent.CreateDynamicMaterialInstance` _cube 0 (`PrimitiveComponent.GetMaterial` _cube 0) "None"))
  (set `self.MaterialRef` _returnvalue))